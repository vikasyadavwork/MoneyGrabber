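; BP_hand is an actor whose Arrow component follows the player's finger across the scene.
; Each tick, while Touch1 is pressed, it traces complex geometry under the finger on the Visibility channel and moves Arrow to the hit X/Y at a fixed world height.
; BeginPlay caches the first BP_hand found, used only by unconnected Cable component lookup code that never runs.
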(event EventBeginPlay
  (bind _returnvalue (Actor|GetActorOfClass "BP_hand_C")))

(event Collision|EventActorBeginOverlap
  (params (OtherActor :type Actor%20Object%20Reference)))

(event EventTick
  (params (DeltaSeconds :type Float%20%28single-precision%29))
  (bind _returnvalue (Game|GetPlayerController 0))
  (bind _biscurrentlypressed (Class|PlayerController|GetInputTouchState _returnvalue "Touch1"))
  (bind _hitresult (Class|PlayerController|GetHitResultUnderFingerbyChannel _returnvalue "Touch1" "TraceTypeQuery1" true))
  (Variables|Default|SetIs%20Currently%20Pressed _biscurrentlypressed)
  (if _biscurrentlypressed
    (Transformation|SetWorldLocation (Variables|Default|GetArrow) (Math|Vector|MakeVector (.x (.location _hitresult)) (.y (.location _hitresult)) 1e+01) false false)))

(fn ConstructionScript)