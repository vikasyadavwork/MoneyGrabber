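; BP_Money is a coin pickup that can be touch-dragged and collected by the player.
; While touched, it moves each tick in XY toward the BP_hand arrow, at a step size scaled by distance.
; When its sphere overlaps a BP_PlayerBase, it destroys itself, has BP_CoinSpawner spawn a new coin and increments the player's TotalMoney.
; The actor-level overlap event only looks up the spawner and has no further effect.
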(event OnInputTouchBegin(StaticMesh)
  (params (FingerIndex :type ETouchIndex%20Enum :default "Touch1") (TouchedComponent :type Primitive%20Component%20Object%20Reference))
  (Variables|Default|SetIsGarbbed true)
  (Actor|GetActorOfClass "/Game/BP_hand.BP_hand_C"))

(event OnComponentBeginOverlap(Sphere)
  (params (OverlappedComponent :type Primitive%20Component%20Object%20Reference) (OtherActor :type Actor%20Object%20Reference) (OtherComp :type Primitive%20Component%20Object%20Reference) (OtherBodyIndex :type Integer) (bFromSweep :type Boolean) (SweepResult :type Hit%20Result%20Structure%20%28by%20ref%29))
  (bind _asbp_player_base (Utilities|Casting|CastToBP_PlayerBase OtherActor))
  (Actor|DestroyActor)
  (bind _returnvalue (Actor|GetActorOfClass "/Game/BP_CoinSpawner.BP_CoinSpawner_C"))
  (Default|SpawnNewCoin _returnvalue)
  (Variables|/Game/BP_PlayerBase.BP_PlayerBase_C|SetTotal%20Money _asbp_player_base (+ (Variables|/Game/BP_PlayerBase.BP_PlayerBase_C|GetTotal%20Money _asbp_player_base) 1)))

(event OnInputTouchEnd(StaticMesh)
  (params (FingerIndex :type ETouchIndex%20Enum :default "Touch1") (TouchedComponent :type Primitive%20Component%20Object%20Reference))
  (Variables|Default|SetIsGarbbed false)
  (Actor|GetActorOfClass "/Game/BP_hand.BP_hand_C"))

(event EventTick
  (params (DeltaSeconds :type Float%20%28single-precision%29))
  (if (Variables|Default|GetIsGarbbed)
    (bind _returnvalue (Actor|GetActorOfClass "/Game/BP_hand.BP_hand_C"))
    (Transformation|AddActorWorldOffset (Math|Vector|MakeVector (.x (* (Math|Vector|Normalize (- (Transformation|GetWorldLocation (Variables|/Game/BP_hand.BP_hand_C|GetArrow _returnvalue)) (Transformation|GetActorLocation))) (Math|Float|MapRangeClamped (Math|Vector|Distance(Vector) (Transformation|GetActorLocation) (Transformation|GetWorldLocation (Variables|/Game/BP_hand.BP_hand_C|GetArrow _returnvalue))) 0.0 8e+02 5.0 3e+01))) (.y (* (Math|Vector|Normalize (- (Transformation|GetWorldLocation (Variables|/Game/BP_hand.BP_hand_C|GetArrow _returnvalue)) (Transformation|GetActorLocation))) (Math|Float|MapRangeClamped (Math|Vector|Distance(Vector) (Transformation|GetActorLocation) (Transformation|GetWorldLocation (Variables|/Game/BP_hand.BP_hand_C|GetArrow _returnvalue))) 0.0 8e+02 5.0 3e+01))) 0.0))))

(event Collision|EventActorBeginOverlap
  (params (OtherActor :type Actor%20Object%20Reference))
  (Utilities|Casting|CastToBP_PlayerBase OtherActor)
  (Actor|GetActorOfClass "/Game/BP_CoinSpawner.BP_CoinSpawner_C"))

(fn ConstructionScript)